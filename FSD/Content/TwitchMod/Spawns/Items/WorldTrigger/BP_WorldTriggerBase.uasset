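; BP_WorldTriggerBase is a base world trigger for the Twitch mod that activates a named spawn group.
; StartTrigger caches the spawn manager, group name, owner ID, target and source actors, and username and message, then sets the trigger's lifespan from the duration.
; A separate SpawnGroup event forwards that cached context to the manager's ActivateSpawnGroupByName; nothing in this base calls it.
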(event Custom|StartTrigger
  (params (SpawnManagert :type Spawn%20Manager%20Object%20Reference) (Duration :type Float%20%28single-precision%29) (SpawnGroup :type String) (Username :type String) (User%20Message :type String) (TargetActor :type Actor%20Object%20Reference) (SourceActor :type Actor%20Object%20Reference) (OwnerID :type Guid%20Structure))
  (Variables|Default|SetSpawnManager SpawnManagert)
  (Variables|Default|SetOwner%20ID OwnerID)
  (Variables|Default|SetInherited%20Actor TargetActor)
  (Variables|Default|SetSource%20Actor SourceActor)
  (Variables|Default|SetSpawn%20Group SpawnGroup)
  (Variables|Default|SetUsername Username)
  (Variables|Default|SetUser%20Message User%20Message)
  (Actor|SetLifeSpan Duration))

(event Custom|SpawnGroup
  (Default|ActivateSpawnGroupbyName (Variables|Default|GetSpawnManager) (Variables|Default|GetSpawn%20Group) (Variables|Default|GetOwner%20ID) (Variables|Default|GetInherited%20Actor) (Variables|Default|GetSource%20Actor) (Variables|Default|GetUsername) (Variables|Default|GetUser%20Message)))

(fn ConstructionScript)