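; Twitch-mod utility spawn that attaches death, damage, proximity and timer triggers to its target actor, each activating a named spawn group from custom properties.
; Health component delegates drive accumulated-damage and death triggers, with EndPlay as death fallback when none exists.
; Tick fires player-proximity and periodic groups behind Delay cooldowns.
; Death groups inherit a BP_DeathProxy spawned at the target's transform; the binder expires after a maximum duration.
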(event Custom|CallbackSpawnEndplay
  (params (Actor :type Actor%20Object%20Reference) (EndPlayReason :type EEndPlayReason%20Enum :default "Destroyed"))
  (if (not (Variables|Default|GetHasDied))
    (Variables|Default|SetHasDied true)
    (CallFunction|SpawnDied)))

(event Custom|CallbackSpawnDeath
  (params (HealthComponent :type Health%20Component%20Base%20Object%20Reference))
  (if (not (Variables|Default|GetHasDied))
    (Variables|Default|SetHasDied true)
    (CallFunction|SpawnDied)))

(event Custom|SpawnDied
  (CallFunction|ActivateGroupbyNameonDeath (.Value (CallFunction|GetCustomProperty "ondeath_group")))
  (Variables|Default|SetHasDied true)
  (CallFunction|DestroyProxy))

(event Custom|CallbackDamageTaken
  (params (Amount :type Float%20%28single-precision%29))
  (CallFunction|SpawnDamageTaken Amount))

(event Custom|SpawnDamageTaken
  (params (Amount :type Float%20%28single-precision%29))
  (bind _output_get (Variables|Default|SetCurrentDmg (+ Amount (Variables|Default|GetCurrentDmg))))
  (if (>= _output_get (Variables|Default|Getdmg_thrshold))
    (Variables|Default|SetCurrentDmg 0.0)
    (Utilities|IsValid (Variables|Default|GetTarget%20Actor)
      (:Is%20Valid
        (CallFunction|ActivateGroupbyName (.Value (CallFunction|GetCustomProperty "ondamaged_group"))))
      (:Is%20Not%20Valid
        (CallFunction|DestroyProxy)))))

(event EventTick
  (params (DeltaSeconds :type Float%20%28single-precision%29))
  (|CallParentFunction DeltaSeconds)
  (if (not (Variables|Default|GetHasDied))
    (Utilities|IsValid (Variables|Default|GetTarget%20Actor)
      (:Is%20Valid
        (Utilities|FlowControl|Sequence
          (:then_0
            (if (not (Variables|Default|GetIsProxOnCooldown))
              (Utilities|IsValid (Class|PlayerCharacterFunctionLibrary|GetNearestPlayerfrom (Transformation|GetActorLocation (Variables|Default|GetTarget%20Actor)) (Variables|Default|GetProxyDistance) true false false)
                (:Is%20Valid
                  (if (not (Utilities|Array|IsEmpty (Variables|Default|Getproxygroup)))
                    (CallFunction|ActivateGroupbyName (Variables|Default|Getproxygroup))
                    (Variables|Default|SetIsProxOnCooldown true)
                    (Utilities|FlowControl|Delay (Variables|Default|Getproxycooldown))
                    (Variables|Default|SetIsProxOnCooldown false))))))
          (:then_1
            (if (not (Variables|Default|GetIsTickOnCooldown))
              (if (not (Utilities|Array|IsEmpty (Variables|Default|Gettickgroup)))
                (CallFunction|ActivateGroupbyName (Variables|Default|Gettickgroup))
                (Variables|Default|SetIsTickOnCooldown true)
                (Utilities|FlowControl|Delay (Variables|Default|Gettickcooldown))
                (Variables|Default|SetIsTickOnCooldown false))))))
      (:Is%20Not%20Valid
        (CallFunction|DestroyProxy)))))

(event EventBeginSpawn
  (params (SpawnManager :type Spawn%20Manager%20Object%20Reference) (SpawnData :type Spawn%20Data%20Structure))
  (|CallParentFunction SpawnManager SpawnData)
  (bind _output_get (Variables|Default|SetTarget%20Actor (Utilities|Struct|BreakSpawnData SpawnData)))
  (if (not (Game|IsActorBeingDestroyed _output_get))
    (Variables|Default|Setproxygroup (.Value (CallFunction|GetCustomProperty "onproximity_group")))
    (Variables|Default|Settickgroup (.Value (CallFunction|GetCustomProperty "ontick_group")))
    (Variables|Default|Setproxycooldown (.Value (CallFunction|GetCustomPropertyFloat "onproximity_cooldown" 5.0)))
    (Variables|Default|Settickcooldown (.Value (CallFunction|GetCustomPropertyFloat "ontick_cooldown" 1.0)))
    (Variables|Default|SetProxyDistance (.Value (CallFunction|GetCustomPropertyFloat "onproximity_distance" 5e+02)))
    (Variables|Default|Setdmg_thrshold (.Value (CallFunction|GetCustomPropertyFloat "ondamaged_threshold" 5e+01)))
    (Actor|Tick|SetActorTickEnabled (or (not (Utilities|Array|IsEmpty (Variables|Default|Getproxygroup))) (not (Utilities|Array|IsEmpty (Variables|Default|Gettickgroup)))))
    (Utilities|FlowControl|Sequence
      (:then_0
        (bind _output_get_2 (Variables|Default|SetHealthComp (Actor|GetComponentbyClass (Variables|Default|GetTarget%20Actor) "/Script/FSD.HealthComponentBase")))
        (Utilities|IsValid _output_get_2
          (:Is%20Valid
            (EventDispatchers|BindEventtoOnDamageTaken (Variables|Default|GetHealthComp) (delegate Custom|CallbackDamageTaken))
            (EventDispatchers|AssignOnDeath (Variables|Default|GetHealthComp) (delegate Custom|CallbackSpawnDeath)))
          (:Is%20Not%20Valid
            (Game|BindEventtoOnEndPlay (Variables|Default|GetTarget%20Actor) (delegate Custom|CallbackSpawnEndplay)))))
      (:then_1
        (Utilities|FlowControl|Delay (.Value (CallFunction|GetCustomPropertyFloat "max_duration" 5e+03)))
        (CallFunction|DestroyProxy)))
    (else
      (CallFunction|DestroyProxy))))

(fn ConstructionScript
  (|CallParentFunction))

(fn ActivateGroupbyNameonDeath
  (params (GroupName :type String))
  (bind _returnvalue (CallFunction|GetSpawnData))
  (bind (_ownerid _sourceactor _username _userinput) (Utilities|Struct|BreakSpawnData _returnvalue))
  (if (not (Utilities|Array|IsEmpty GroupName))
    (bind _returnvalue_2 (Game|SpawnActorfromClass "/Game/TwitchMod/Spawns/Items/BP_DeathProxy.BP_DeathProxy_C" (Transformation|GetActorTransform (Variables|Default|GetTarget%20Actor)) "AlwaysSpawn" 0 0))
    (Default|ActivateSpawnGroupbyName (CallFunction|GetSpawnManager) GroupName _ownerid _returnvalue_2 _sourceactor _username _userinput)))

(fn ActivateGroupbyName
  (params (GroupName :type String))
  (bind _returnvalue (CallFunction|GetSpawnData))
  (bind (_ownerid _sourceactor _username _userinput) (Utilities|Struct|BreakSpawnData _returnvalue))
  (if (not (Utilities|Array|IsEmpty GroupName))
    (Default|ActivateSpawnGroupbyName (CallFunction|GetSpawnManager) GroupName _ownerid (Variables|Default|GetTarget%20Actor) _sourceactor _username _userinput)))