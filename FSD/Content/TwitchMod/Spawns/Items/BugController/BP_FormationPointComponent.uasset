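; BP_FormationPointComponent is a scene component marking one slot in a swarm bug formation and steering its assigned bug toward it.
; StartMovement begins pathfinder movement, unless the bug is already moving, toward the slot's world location pushed ahead along the given direction.
; UpdateDestination refreshes that target with its own carrot offset, so the bug chases a point leading the slot.
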(event Custom|UpdateDestination
  (params (Direction :type Vector))
  (Utilities|IsValid (Variables|Default|GetSwarmBugRef)
    (:Is%20Valid
      (Class|DeepPathfinderMovement|UpdateDestination (Variables|/Script/FSD.DeepPathfinderCharacter|GetPathfinderMovement (Variables|Default|GetSwarmBugRef)) (+ (Transformation|GetWorldLocation) (* Direction (Variables|Default|GetCarrotOffsetUpdate)))))))

(event Custom|StartMovement
  (params (Direction :type Vector))
  (Utilities|IsValid (Variables|Default|GetSwarmBugRef)
    (:Is%20Valid
      (if (Utilities|Enum|NotEqual(Enum) (Class|DeepPathfinderMovement|GetMovementState (Variables|/Script/FSD.DeepPathfinderCharacter|GetPathfinderMovement (Variables|Default|GetSwarmBugRef))) "Moving")
        (Class|DeepPathfinderMovement|StartMoveto (Variables|/Script/FSD.DeepPathfinderCharacter|GetPathfinderMovement (Variables|Default|GetSwarmBugRef)) (+ (Transformation|GetWorldLocation) (* Direction (Variables|Default|GetCarrotOffsetStart))) 5.0)))))