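; BP_BugNameplateComponent is a widget component that shows a text nameplate for bugs in the Twitch mod.
; Every tick it rotates in world space to face the local player's camera, giving a billboard effect.
; SetNameplateText forwards new text to its WB_BugNameplate widget, provided that widget is valid and of that class.
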(event EventBeginPlay
  (CallFunction|GetLocalPlayer))

(event EventTick
  (params (DeltaSeconds :type Float%20%28single-precision%29))
  (bind _returnvalue (CallFunction|GetLocalPlayer))
  (Transformation|SetWorldRotation self (Math|Rotator|FindLookatRotation (Transformation|GetWorldLocation self) (Camera|GetCameraLocation (Variables|/Script/Engine.PlayerController|GetPlayerCameraManager _returnvalue))) false false))

(fn SetNameplateText
  (params (NewText :type String))
  (bind _returnvalue (UserInterface|GetUserWidgetObject))
  (Utilities|IsValid _returnvalue
    (:Is%20Valid
      (bind _aswb_bug_nameplate (Utilities|Casting|CastToWB_BugNameplate _returnvalue))
      (Default|SetNameplateText _aswb_bug_nameplate NewText))))