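; BP_TwitchReplicationHelper is a Twitch mod network helper exposing events that change spawned actors' appearance and play sounds, named as Server and Multicast calls.
; The material event creates one dynamic instance and applies it at a given slot to static and skeletal mesh components, skipping hidden ones and meshes named "Sphere".
; The other events set an actor's scale and spawn a sound attached to a component.
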(event Custom|Server_SetActorScale
  (params (Spawn :type Actor%20Object%20Reference) (NewScale :type Vector))
  (Transformation|SetActorScale3D Spawn NewScale))

(event Custom|Server_ApplyMaterialToMesh
  (params (Spawn :type Actor%20Object%20Reference) (Material :type Material%20Interface%20Object%20Reference) (SlotIndex :type Integer))
  (bind _returnvalue (Rendering|Material|CreateDynamicMaterialInstance Material "None" "None" :!class /Script/Engine.KismetMaterialLibrary))
  (for _array_element (Actor|GetComponentsByClass Spawn "/Script/Engine.StaticMeshComponent")
    (if (not (Variables|/Script/Engine.SceneComponent|GetbHiddenInGame _array_element))
      (if (not (Utilities|Enum|Equal(Enum) (Utilities|GetObjectName (Variables|/Script/Engine.StaticMeshComponent|GetStaticMesh _array_element)) "Sphere"))
        (Rendering|Material|SetMaterial _array_element SlotIndex _returnvalue))))
  (for _array_element_2 (Actor|GetComponentsByClass Spawn "/Script/Engine.SkeletalMeshComponent")
    (if (not (Variables|/Script/Engine.SceneComponent|GetbHiddenInGame _array_element_2))
      (if (not (Utilities|Enum|Equal(Enum) (Utilities|GetObjectName (Variables|/Script/Engine.SkinnedMeshComponent|GetSkeletalMesh _array_element_2)) "Sphere"))
        (Rendering|Material|SetMaterial _array_element_2 SlotIndex _returnvalue)))))

(event Custom|Multicast_PlaySound
  (params (Sound :type Sound%20Base%20Object%20Reference) (AttachToComponent :type Scene%20Component%20Object%20Reference) (VolumeMultiplier :type Float%20%28single-precision%29) (PitchMultiplier :type Float%20%28single-precision%29))
  (Audio|SpawnSoundAttached Sound AttachToComponent "None" "0, 0, 0" "0, 0, 0" "KeepRelativeOffset" false VolumeMultiplier PitchMultiplier 0.0 0 0))

(fn ConstructionScript)