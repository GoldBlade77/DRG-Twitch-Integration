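; Twitch mod notifications module that queues styled messages and shows them one at a time on the HUD, optionally echoing them to chat.
; Styles load from a data table, filtered by Steam ID restrictions, and supply each message's widget class.
; A looping timer pulls from the queue when idle, with high-priority messages inserted first; disabling the module pauses it.
; Widgets retry adding to the viewport until present, then are removed after duration and cleanup delays.
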(event Custom|CheckForNewMessage
  (if (not (Variables|Default|GetIsShowingNotification))
    (CallFunction|NextMessage)))

(event Custom|Next%20Message
  (if (Utilities|Array|IsValidIndex (Variables|Default|GetNotificationQueue))
    (Variables|Default|SetCurrentNotification (Utilities|Array|Get(acopy) (Variables|Default|GetNotificationQueue)))
    (Utilities|Array|RemoveIndex (Variables|Default|GetNotificationQueue))
    (Variables|Default|SetIsShowingNotification true)
    (if (Variables|/Game/TwitchMod/Settings/SAV_TwitchSettings.SAV_TwitchSettings_C|GetShowNotificationsInChat (CallFunction|GetModSettings))
      (CallFunction|SendChatMessage "Twitch" (Utilities|Struct|BreakNotificationData (Variables|Default|GetCurrentNotification)) "Streamer"))
    (if (Variables|/Game/TwitchMod/Settings/SAV_TwitchSettings.SAV_TwitchSettings_C|GetShowNotificationsOnHUD (CallFunction|GetModSettings))
      (bind _returnvalue (UserInterface|CreateWidget (.WidgetClass (Utilities|Struct|BreakNotificationData (Variables|Default|GetCurrentNotification)))))
      (bind _output_get (Variables|Default|SetCurrentWidget _returnvalue))
      (Utilities|AddWidgettoViewport _output_get 500)
      (Class|INotificationWidget|BeginNotification(Message) _output_get self (.Username (Utilities|Struct|BreakNotificationData (Variables|Default|GetCurrentNotification))) (.Message (Utilities|Struct|BreakNotificationData (Variables|Default|GetCurrentNotification))) (.Duration (Utilities|Struct|BreakNotificationData (Variables|Default|GetCurrentNotification))))
      (Utilities|FlowControl|RetriggerableDelay (.Duration (Utilities|Struct|BreakNotificationData (Variables|Default|GetCurrentNotification))))
      (Class|INotificationWidget|NotificationFinished(Message) (Variables|Default|GetCurrentWidget) (Math|Float|Truncate (Variables|Default|GetCleanupTime)))
      (Utilities|FlowControl|RetriggerableDelay (Variables|Default|GetCleanupTime))
      (Widget|RemovefromParent (Variables|Default|GetCurrentWidget))
      (Variables|Default|SetIsShowingNotification false)
      (else
        (Variables|Default|SetIsShowingNotification false)))))

(event EventLoadModule
  (params (Mod :type Mod%20Twitch%20Mod%20Object%20Reference%20%28by%20ref%29))
  (|CallParentFunction Mod)
  (Utilities|LoadDefaultNotificationStyles
    (:Completed
      (bind _returnvalue (Utilities|Time|SetTimerbyEvent (delegate Custom|CheckForNewMessage) 0.5 true))
      (Variables|Default|SetQueueTimer _returnvalue)
      (Default|CallOnModuleLoaded))))

(event EventEnableModule
  (|CallParentFunction)
  (CallFunction|ResumeNotifications))

(event EventAddNotificationStyle
  (params (ID :type Name :default "None") (Name :type String) (Description :type String) (Thumbnail :type Texture%202D%20Object%20Reference) (WidgetClass :type User%20Widget%20Class%20Reference) (RestrictToSteamIDs :type Array%20of%20Strings))
  (bind _notificationstyle (Utilities|Struct|MakeNotificationStyle ID Name Description Thumbnail WidgetClass RestrictToSteamIDs))
  (bind _returnvalue (CallFunction|CanAccessRestrictedSteamIDs RestrictToSteamIDs true))
  (if _returnvalue
    (Utilities|Array|Add (Variables|Default|GetNotificationStyles) _notificationstyle)
    (Default|CallOnNotificationStyleAdded _notificationstyle)))

(event EventDisableModule
  (|CallParentFunction)
  (CallFunction|PauseNotifications))

(event EventUpdateModule
  (|CallParentFunction)
  (if (CallFunction|IsModuleEnabled)
    _))

(fn SendNotification
  (params (HighPriority :type Boolean) (StyleID :type Name) (Username :type String) (Message :type String) (Duration :type Float%20%28single-precision%29))
  (bind _returnvalue (CallFunction|GetModSettings))
  (bind (_returnvalue_2 _notificationstyle) (CallFunction|GetNotificationStyle StyleID))
  (if _returnvalue_2
    (if (or (Variables|/Game/TwitchMod/Settings/SAV_TwitchSettings.SAV_TwitchSettings_C|GetShowNotificationsOnHUD _returnvalue) (Variables|/Game/TwitchMod/Settings/SAV_TwitchSettings.SAV_TwitchSettings_C|GetShowNotificationsInChat _returnvalue))
      (if HighPriority
        (Utilities|Array|Insert (Variables|Default|GetNotificationQueue) (Utilities|Struct|MakeNotificationData (Utilities|Struct|BreakNotificationStyle _notificationstyle) Username Message Duration))
        (else
          (Utilities|Array|Add (Variables|Default|GetNotificationQueue) (Utilities|Struct|MakeNotificationData (Utilities|Struct|BreakNotificationStyle _notificationstyle) Username Message Duration)))))))

(fn ClearNotifications
  (Utilities|Array|Clear (Variables|Default|GetNotificationQueue)))

(fn PauseNotifications
  (Utilities|Time|PauseTimerbyHandle (Variables|Default|GetQueueTimer)))

(fn ResumeNotifications
  (Utilities|Time|UnpauseTimerbyHandle (Variables|Default|GetQueueTimer)))

(fn GetNotificationStyle
  (params (StyleID :type Name))
  (for _array_element (Variables|Default|GetNotificationStyles)
    (if (Utilities|Name|Equal(Name) (Utilities|Struct|BreakNotificationStyle _array_element) StyleID)
      (return true _array_element)))
  (return false ""))