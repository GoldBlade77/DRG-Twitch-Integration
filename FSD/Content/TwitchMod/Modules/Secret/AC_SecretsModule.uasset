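; Twitch mod module component that handles secret chat commands restricted to an allowed-user list.
; For allowed users, a command found in the SecretSpawns map spawns its mapped actor class and calls PlaySecret with the mod, command and arguments.
; Otherwise, one hardcoded owner username can add, remove or reset allowed users through admin commands, with names lowercased for matching.
; An IsServer check exists in the graph but is disconnected.
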(event Custom|TryPlaySecretCommand
  (params (Username :type String) (Command :type String) (Args :type Array%20of%20Strings))
  (bind _output (Utilities|Array|Get(acopy) Args))
  (bind _secretspawns (Variables|Default|GetSecretSpawns))
  (bind (_value _returnvalue) (Utilities|Map|Find _secretspawns Command))
  (bind _returnvalue_2 (Utilities|String|ToLower _output))
  (if (CallFunction|IsUserAllowed Username)
    (if _returnvalue
      (bind _returnvalue_3 (Game|SpawnActorfromClass _value (Math|Transform|MakeTransform "0, 0, 0" "0, 0, 0" "1,1,1") "AlwaysSpawn" 0 0))
      (Default|PlaySecret _returnvalue_3 (CallFunction|GetTwitchMod) Command Args)
      (else
        (if (Utilities|Enum|Equal(Enum) Username "goldbl4d3") :!label _label
          (switch string Command
            (:s_add_user
              (Utilities|Array|Add (Variables|Default|GetAllowedUsers) _returnvalue_2))
            (:s_remove_user
              (Utilities|Array|RemoveItem (Variables|Default|GetAllowedUsers) _returnvalue_2))
            (:s_reset
              (Utilities|Array|Clear (Variables|Default|GetAllowedUsers))
              (Utilities|Array|Add (Variables|Default|GetAllowedUsers) "goldbl4d3"))))))
    (else
      (goto _label))))

(event EventLoadModule
  (params (Mod :type Mod%20Twitch%20Mod%20Object%20Reference%20%28by%20ref%29))
  (|CallParentFunction Mod)
  (Default|CallOnModuleLoaded))

(fn IsUserAllowed
  (params (Username :type String%20%28by%20ref%29))
  (return (Utilities|Array|ContainsItem (Variables|Default|GetAllowedUsers) (Utilities|String|ToLower Username))))