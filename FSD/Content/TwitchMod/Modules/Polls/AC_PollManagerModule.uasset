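; Twitch mod module that queues and runs timed two-choice viewer polls, broadcasting the winning choice and its item configs.
; A looping timer starts queued polls when idle, spawning each widget from data-table styles gated by Steam ID.
; Ballots allow one vote per username and update the widget's tallies until countdown or cancellation.
; Ties, and empty polls with auto-vote, always yield A because both random-pick branches select A.
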(event Custom|CheckForNewPolls
  (Utilities|SwitchonPollState
    (:Inactive
      (CallFunction|BeginNextPoll))))

(event Custom|EndPoll
  (params (bCancelled :type Boolean))
  (Utilities|SwitchonPollState
    (:Active
      (Utilities|FlowControl|DoOnce false :!label _label
        (:Completed
          (Utilities|Time|ClearandInvalidateTimerbyHandle (Variables|Default|GetCountdownTimer))
          (if bCancelled
            (Class|IPollWidget|PollFinished(Message) (Variables|Default|GetCurrentPollWidget) false "NewEnumerator0" "" (Variables|Default|GetPollCleanupTime))
            (else
              (bind (_success _winner _winningchoice _itemconfigs) (CallFunction|CalculatePollWinner))
              (Class|IPollWidget|PollFinished(Message) (Variables|Default|GetCurrentPollWidget) _success _winner _winningchoice (Variables|Default|GetPollCleanupTime))
              (if _success
                (Default|CallOnSuccessfulPoll (Utilities|Struct|BreakPollData (Variables|Default|GetCurrentPoll)) _winner _winningchoice _itemconfigs))))
          (Utilities|FlowControl|Delay (Math|Conversions|ToFloat(Integer) (Variables|Default|GetPollCleanupTime)))
          (Widget|RemovefromParent (Variables|Default|GetCurrentPollWidget))
          (Variables|Default|SetCurrentPollWidget 0)
          (Variables|Default|SetIsPollActive false)
          (Default|CallOnPollFinished)
          (goto _label Reset))))))

(event Custom|TimeRemainingElapsed
  (bind _result (Math|Integer|DecrementInt (Variables|Default|GetTimeRemaining))
    (:%20%20
      (Class|IPollWidget|UpdateTime(Message) (Variables|Default|GetCurrentPollWidget) _result)
      (if (<= _result 0)
        (Utilities|Time|ClearandInvalidateTimerbyHandle (Variables|Default|GetCountdownTimer))
        (CallFunction|EndPoll false)))))

(event Custom|BeginNextPoll
  (Utilities|SwitchonPollState
    (:Inactive
      (Variables|Default|SetCurrentPoll "")
      (Variables|Default|SetTimeRemaining 0)
      (Utilities|Time|ClearandInvalidateTimerbyHandle (Variables|Default|GetCountdownTimer))
      (CallFunction|ClearVotes)
      (if (Utilities|Array|IsValidIndex (Variables|Default|GetPollQueue))
        (Variables|Default|SetIsPollActive true)
        (Variables|Default|SetCurrentPoll (Utilities|Array|Get(acopy) (Variables|Default|GetPollQueue)))
        (Utilities|Array|RemoveIndex (Variables|Default|GetPollQueue))
        (bind _returnvalue (UserInterface|CreateWidget (.WidgetClass (Utilities|Struct|BreakPollData (Variables|Default|GetCurrentPoll)))))
        (bind _output_get (Variables|Default|SetCurrentPollWidget _returnvalue))
        (Class|IPollWidget|BeginPoll(Message) _output_get (.Title (Utilities|Struct|BreakPollData (Variables|Default|GetCurrentPoll))) (.ChoiceA (Utilities|Struct|BreakPollData (Variables|Default|GetCurrentPoll))) (.ChoiceB (Utilities|Struct|BreakPollData (Variables|Default|GetCurrentPoll))) (.IconA (Utilities|Struct|BreakPollData (Variables|Default|GetCurrentPoll))) (.IconB (Utilities|Struct|BreakPollData (Variables|Default|GetCurrentPoll))) (.Duration (Utilities|Struct|BreakPollData (Variables|Default|GetCurrentPoll))))
        (Variables|Default|SetTimeRemaining (.Duration (Utilities|Struct|BreakPollData (Variables|Default|GetCurrentPoll))))
        (UserInterface|Viewport|AddtoViewport _output_get 4)
        (Utilities|FlowControl|Delay 1.0)
        (bind _returnvalue_2 (Utilities|Time|SetTimerbyEvent (delegate Custom|TimeRemainingElapsed) 1.0 true))
        (Variables|Default|SetCountdownTimer _returnvalue_2)))))

(event Custom|StartPollQueue
  (bind _returnvalue (Utilities|Time|SetTimerbyEvent (delegate Custom|CheckForNewPolls) 1.0 true))
  (Variables|Default|SetQueueTimer _returnvalue))

(event Custom|StopPollQueue
  (params (StopActivePoll :type Boolean))
  (Utilities|Time|ClearandInvalidateTimerbyHandle (Variables|Default|GetQueueTimer))
  (if StopActivePoll
    (Utilities|SwitchonPollState
      (:Active
        (CallFunction|EndPoll true)))))

(event EventAddPollStyle
  (params (ID :type Name :default "None") (Name :type String) (Description :type String) (Thumbnail :type Texture%202D%20Object%20Reference) (WidgetClass :type User%20Widget%20Class%20Reference) (RestrictToSteamIDs :type Array%20of%20Strings))
  (bind _pollstyle (Utilities|Struct|MakePollStyle ID Name Description Thumbnail WidgetClass RestrictToSteamIDs))
  (bind _returnvalue (CallFunction|CanAccessRestrictedSteamIDs RestrictToSteamIDs true))
  (if _returnvalue
    (Utilities|Array|Add (Variables|Default|GetPollStyles) _pollstyle)
    (Default|CallOnPollStyleAdded _pollstyle)))

(event EventEnableModule
  (|CallParentFunction))

(event EventDisableModule
  (|CallParentFunction))

(event EventUpdateModule
  (|CallParentFunction)
  (if (CallFunction|IsModuleEnabled)
    _))

(event EventLoadModule
  (params (Mod :type Mod%20Twitch%20Mod%20Object%20Reference%20%28by%20ref%29))
  (|CallParentFunction Mod)
  (Utilities|LoadDefaultPollStyles
    (:Completed
      (Default|CallOnModuleLoaded))))

(event EventCancelActivePoll
  (CallFunction|EndPoll true))

(fn StartNewPoll
  (params (ClearQueue :type Boolean) (StyleID :type Name) (Title :type String) (ChoiceA :type String) (ChoiceB :type String) (IconA :type Texture%202D%20Object%20Reference) (IconB :type Texture%202D%20Object%20Reference) (Duration :type Integer) (ItemConfigs_A :type Array%20of%20Spawn%20Item%20Config%20Structures) (ItemConfigs_B :type Array%20of%20Spawn%20Item%20Config%20Structures))
  (if ClearQueue
    (Utilities|Array|Clear (Variables|Default|GetPollQueue)))
  (bind (_returnvalue _style) (CallFunction|GetPollStyle StyleID))
  (if _returnvalue
    (Utilities|Array|Add (Variables|Default|GetPollQueue) (Utilities|Struct|MakePollData (Utilities|Struct|BreakPollStyle _style) Title ChoiceA ChoiceB IconA IconB Duration ItemConfigs_A ItemConfigs_B))))

(fn AddBallot
  (params (Username :type String) (Choice :type EPollChoice%20Enum :default "NewEnumerator0"))
  (bind _returnvalue (Utilities|String|ToLower Username))
  (bind _pollballot (Utilities|Struct|MakePollBallot _returnvalue Choice))
  (bind _choice (Utilities|Struct|BreakPollBallot _pollballot))
  (if (not (CallFunction|HasViewerAlreadyVoted _returnvalue))
    (Utilities|Array|Add (Variables|Default|GetCurrentBallots) _pollballot)
    (Default|CallOnBallotAdded Username _choice)
    (switch Utilities|FlowControl|Switch|SwitchonEPollChoice _choice
      (:NewEnumerator0
        (Math|Integer|IncrementInt (Variables|Default|GetVoteTallyA)
          (:%20%20
            _)))
      (:NewEnumerator1
        (Math|Integer|IncrementInt (Variables|Default|GetVoteTallyB)
          (:%20%20
            _))))
    (bind _currentpollwidget (Variables|Default|GetCurrentPollWidget)
      (:then
        (Class|IPollWidget|UpdateTally(Message) _currentpollwidget (Variables|Default|GetVoteTallyA) (Variables|Default|GetVoteTallyB)))
      (:else))))

(fn ClearVotes
  (Utilities|Array|Clear (Variables|Default|GetCurrentBallots))
  (Variables|Default|SetVoteTallyA 0)
  (Variables|Default|SetVoteTallyB 0)
  (bind _currentpollwidget (Variables|Default|GetCurrentPollWidget)
    (:then
      (Class|IPollWidget|UpdateTally(Message) _currentpollwidget))
    (:else)))

(fn HasViewerAlreadyVoted
  (params (Username :type String))
  (for _array_element (Variables|Default|GetCurrentBallots)
    (if (Utilities|Enum|Equal(Enum) (Utilities|Struct|BreakPollBallot _array_element) Username)
      (return true)))
  (return false))

(fn CalculatePollWinner
  (bind _currentpoll (Variables|Default|GetCurrentPoll))
  (bind (_widgetclass _title _choicea _choiceb _icona _iconb _duration _itemconfigs_a _itemconfigs_b) (Utilities|Struct|BreakPollData _currentpoll))
  (if (== (+ (Variables|Default|GetVoteTallyA) (Variables|Default|GetVoteTallyB)) 0)
    (if (Variables|/Game/TwitchMod/Settings/SAV_TwitchSettings.SAV_TwitchSettings_C|GetPollAutoVote (CallFunction|GetModSettings))
      _
      (else
        (return false "NewEnumerator0" "" 0)))
    (else
      (Math|Integer|CompareInt (Variables|Default|GetVoteTallyA) (Variables|Default|GetVoteTallyB)
        (:>
          (return true "NewEnumerator0" _choicea _itemconfigs_a))
        (:==
          _)
        (:<
          (return true "NewEnumerator1" _choiceb _itemconfigs_b)))))
  (bind _output_get (LocalVariables|SetNewLocalVar_0 (select (Math|Random|RandomBool) "NewEnumerator0" "NewEnumerator0")))
  (return true _output_get (Utilities|Select :Index _output_get :NewEnumerator0 _choicea :NewEnumerator1 _choiceb) (Utilities|Select :Index _output_get :NewEnumerator0 _itemconfigs_a :NewEnumerator1 _itemconfigs_b)))

(fn GetPollStyle
  (params (StyleID :type Name))
  (for _array_element (Variables|Default|GetPollStyles)
    (if (Utilities|Name|Equal(Name) (Utilities|Struct|BreakPollStyle _array_element) StyleID)
      (return true _array_element)))
  (return false ""))

(fn GetChoicefromCommand
  (params (Command :type String))
  (switch string (Utilities|String|TrimTrailing (Utilities|String|Trim (Utilities|String|ToLower Command)))
    (:Default
      (return false "NewEnumerator0"))
    (:a
      (return true "NewEnumerator0"))
    (:b
      (return true "NewEnumerator1"))))