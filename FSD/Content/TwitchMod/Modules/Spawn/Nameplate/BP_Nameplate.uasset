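; Replicated nameplate actor from the TwitchMod Spawn module that attaches to a parent actor and shows text and an icon.
; Setup applies a configurable widget class, and setters and OnRep handlers push content changes to the widget.
; Tick turns the widget toward the local player's camera.
; It hides and destroys itself on the parent's death, while a looping timer cleans it up if the parent becomes invalid.
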(event Custom|OwnerDied
  (params (HealthComponent :type Health%20Component%20Base%20Object%20Reference))
  (CallFunction|HideNameplate)
  (CallFunction|DestroyNameplate))

(event Custom|CheckCleanup
  (Utilities|IsValid (Variables|Default|GetParentActor)
    (:Is%20Not%20Valid
      (CallFunction|DestroyNameplate))))

(event Custom|UpdateWidget
  (bind _nameplatewidget (Variables|Default|GetNameplateWidget)
    (:then
      (Class|INameplateWidget|UpdateNameplateWidget(Message) _nameplatewidget (Variables|Default|GetText) (Variables|Default|GetIcon) (Variables|Default|GetShowIcon) (Variables|Default|GetTextColorOverride)))
    (:else)))

(event Custom|SetupNameplate
  (params (Parent :type Actor%20Object%20Reference) (WidgetClass :type User%20Widget%20Class%20Reference) (OffsetRelative :type Vector) (Text :type String) (Icon :type Texture%202D%20Object%20Reference) (ShowIcon :type Boolean) (TextColorOverride :type Linear%20Color%20Structure))
  (Variables|Default|SetParentActor Parent)
  (Variables|Default|SetWidgetClass WidgetClass)
  (Variables|Default|SetOffsetRelative OffsetRelative)
  (Variables|Default|SetText Text)
  (Variables|Default|SetIcon Icon)
  (Variables|Default|SetShowIcon ShowIcon)
  (Variables|Default|SetTextColorOverride TextColorOverride)
  (CallFunction|ApplyWidgetClass (Variables|Default|GetWidgetClass))
  (CallFunction|UpdateWidget)
  (Actor|Tick|SetActorTickEnabled true)
  (bind _returnvalue (Utilities|Time|SetTimerbyEvent (EventDispatchers|CreateEvent :!event Custom|CheckCleanup) 5.0 true))
  (Variables|Default|SetCleanupTimer _returnvalue)
  (Transformation|SetActorLocation (Variables|Default|GetOffsetRelative) false false)
  (Transformation|AttachActorToActor self (Variables|Default|GetParentActor) "None" "KeepRelative" "KeepRelative" "KeepWorld" false)
  (bind _output_get (Variables|Default|SetParentHealth (Actor|GetComponentbyClass (Variables|Default|GetParentActor) "/Script/FSD.HealthComponentBase")))
  (Utilities|IsValid _output_get
    (:Is%20Valid
      (EventDispatchers|BindEventtoOnDeath (Variables|Default|GetParentHealth) (EventDispatchers|CreateEvent :!event Custom|OwnerDied)))))

(event EventBeginPlay
  (bind _player (Utilities|WaitforLocalPlayer)
    (:Completed
      (Variables|Default|SetLocalPlayer _player)
      (if (not (Networking|IsServer))
        (Actor|Tick|SetActorTickEnabled true)))))

(event EventSetIcon
  (params (Icon :type Texture%202D%20Object%20Reference))
  (Variables|Default|SetIcon Icon)
  (CallFunction|UpdateWidget))

(event EventSetTextColorOverride
  (params (TextColorOverride :type Linear%20Color%20Structure))
  (Variables|Default|SetTextColorOverride TextColorOverride)
  (CallFunction|UpdateWidget))

(event EventTick
  (params (DeltaSeconds :type Float%20%28single-precision%29))
  (bind _widget (Variables|Default|GetWidget)
    (:then
      (Transformation|SetWorldRotation _widget (Math|Rotator|FindLookatRotation (Transformation|GetWorldLocation (Variables|Default|GetWidget)) (Camera|GetCameraLocation (Variables|/Script/Engine.PlayerController|GetPlayerCameraManager (Variables|Default|GetLocalPlayer)))) false false))
    (:else)))

(event EventSetText
  (params (Text :type String))
  (Variables|Default|SetText Text)
  (CallFunction|UpdateWidget))

(fn ConstructionScript)

(fn HideNameplate
  (Rendering|SetVisibility (Variables|Default|GetWidget) false false))

(fn ShowNameplate
  (Rendering|SetVisibility (Variables|Default|GetWidget) true false))

(fn DestroyNameplate
  (Networking|SwitchHasAuthority
    (:Authority
      (Actor|Tick|SetActorTickEnabled false)
      (if (not (Game|IsActorBeingDestroyed (Variables|Default|GetParentActor)))
        (Actor|DestroyActor)))))

(fn OnRepShowIcon
  (CallFunction|UpdateWidget))

(fn OnRepText
  (CallFunction|UpdateWidget))

(fn OnRepTextColor
  (CallFunction|UpdateWidget))

(fn OnRepIcon
  (CallFunction|UpdateWidget))

(fn OnRepWidgetClass
  (CallFunction|ApplyWidgetClass (Variables|Default|GetWidgetClass)))

(fn ApplyWidgetClass
  (params (Class :type User%20Widget%20Class%20Reference))
  (if (Utilities|IsValidClass Class)
    (bind _returnvalue (UserInterface|CreateWidget Class))
    (bind _output_get (Variables|Default|SetNameplateWidget _returnvalue))
    (UserInterface|SetWidget (Variables|Default|GetWidget) _output_get)
    (CallFunction|UpdateWidget)))

(fn GetNameplateWidget
  (bind _asinameplate_widget (Utilities|Casting|CastToINameplateWidget (Variables|Default|GetNameplateWidget)))
  (return _asinameplate_widget))