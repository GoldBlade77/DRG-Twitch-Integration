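; BP_Gravesite is a gravesite actor in the TwitchMod chat-control spawn module that carves terrain and raises a gravestone.
; On BeginPlay it carves terrain using its CarveMesh shape and dirt material, then a timeline lifts the gravestone from below.
; CleanupGrave waits a random sub-second delay, sinks the stone with a second timeline, then destroys the actor.
; All_PlayRiseEffects runs the particles briefly as a separate event.
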(event Custom|CleanupGrave
  (Variables|Default|SetStartingLocationRel "-173.000000, 0,-10.000000")
  (Utilities|FlowControl|Delay (Math|Random|RandomFloatinRange 0.0 1.0))
  (bind _zoffset (Timeline|Timeline_0 PlayFromStart)
    (:Update
      (Transformation|SetRelativeLocation (Variables|Default|GetGraveStoneMesh) (- (Variables|Default|GetStartingLocationRel) (Math|Vector|MakeVector 0.0 0.0 _zoffset)) false false))
    (:Finished
      (Actor|DestroyActor))))

(event Custom|All_PlayRiseEffects
  (Components|Activation|Activate (Variables|Default|GetParticles) false)
  (Utilities|FlowControl|Delay 3.0)
  (Components|Activation|Deactivate (Variables|Default|GetParticles)))

(event EventBeginPlay
  (bind _carvemesh (Variables|Default|GetCarveMesh))
  (CallFunction|CarveTerrain (Variables|/Script/Engine.StaticMeshComponent|GetStaticMesh _carvemesh) "/Game/Landscape/Materials/TM_Dirt.TM_Dirt" "ReplaceAll" (Transformation|GetWorldTransform _carvemesh) 5.0)
  (Variables|Default|SetStartingLocationRel "-173.000000, 0,-110.000000")
  (bind _zoffset (Timeline|Timeline_1 PlayFromStart)
    (:Update
      (Transformation|SetRelativeLocation (Variables|Default|GetGraveStoneMesh) (+ (Variables|Default|GetStartingLocationRel) (Math|Vector|MakeVector 0.0 0.0 _zoffset)) false false))))

(fn ConstructionScript)