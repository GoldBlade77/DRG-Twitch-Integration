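; BP_WorldTriggerBase is a base actor for timed world triggers in the Twitch mod's item spawn module.
; StartTrigger stores the spawn manager, state container, parent context, group name and user details, then sets the actor's lifespan from the given duration.
; The SpawnGroup event asks AC_SpawnManagerModule to spawn the named item group, passing the user details, parent context and local player character.
; Nothing in this Blueprint calls SpawnGroup itself.
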(event Custom|StartTrigger
  (params (SpawnManager :type I%20Spawn%20Manager%20Interface) (StateContainer :type Object%20Object%20Reference) (ParentContext :type Actor%20Object%20Reference) (Duration :type Float%20%28single-precision%29) (SpawnGroup :type String) (Username :type String) (User%20Message :type String))
  (Variables|Default|SetSpawn%20Manager SpawnManager)
  (Variables|Default|SetState%20Container StateContainer)
  (Variables|Default|SetParent%20Context ParentContext)
  (Variables|Default|SetSpawn%20Group SpawnGroup)
  (Variables|Default|SetUsername Username)
  (Variables|Default|SetUser%20Message User%20Message)
  (Actor|SetLifeSpan Duration))

(event Custom|SpawnGroup
  (bind _asac_spawn_manager_module (Utilities|Casting|CastToAC_SpawnManagerModule (Variables|Default|GetSpawn%20Manager)))
  (Default|SpawnItemGroupswithName _asac_spawn_manager_module (Variables|Default|GetSpawn%20Group) (Variables|Default|GetUsername) (Variables|Default|GetUser%20Message) (Variables|Default|GetParent%20Context) (CallFunction|GetLocalPlayerCharacter)))

(fn ConstructionScript)