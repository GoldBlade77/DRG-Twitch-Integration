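; Twitch mod actor that lets a player pilot a spawned bug and summonable swarm while their character is hidden and invulnerable.
; It attaches to the AI-unpossessed bug once the client accepts, otherwise timing out.
; Local input drives server events for pathfinder movement, formation-offset swarming and cooldown-gated attacks through named components with configurable sphere-overlap targeting.
; Primary bug death kills the swarm and destroys the controller, restoring the player there.
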(event Custom|SERVER_PrimaryAttack
  (params (CameraTransform :type Transform))
  (if (Variables|Controller|BugAttacks|GetCanUsePrimaryAttack)
    (CallFunction|Attack (CallFunction|GetPrimaryBug) (Variables|Controller|BugAttacks|GetPrimaryAttackName) (Variables|Controller|BugAttacks|GetPrimaryAttackRadius) (Variables|Controller|BugAttacks|GetPrimaryAttackDistance) (Variables|Controller|BugAttacks|GetPrimaryTargetingMethod) (Variables|Controller|BugAttacks|GetPrimaryTargetingRule) CameraTransform)
    (Variables|Controller|BugAttacks|SetCanUsePrimaryAttack false)
    (Utilities|Time|SetTimerbyEvent (delegate Custom|EnablePrimaryAttack) (Variables|Controller|BugAttacks|GetPrimaryAttackCooldown))))

(event Custom|SwarmCooldownEnd
  (Variables|Controller|Swarm|SetCanSummonSwarm true))

(event Custom|BugDied
  (if (not (Variables|Private|GetIsDead))
    (Variables|Private|SetIsDead true)
    (CallFunction|KillSwarm)
    (Utilities|FlowControl|Delay (Variables|Controller|GetCleanupDelay))
    (Actor|DestroyActor)))

(event Custom|PrimaryBugDestroyed
  (params (DestroyedActor :type Actor%20Object%20Reference))
  (CallFunction|BugDied))

(event Custom|SERVER_AcceptController
  (Variables|private|SetClientAccepted true)
  (CallFunction|SetPlayerGodMode true true true true)
  (bind _spawnedbug (CallFunction|SpawnBugAttached (+ (Transformation|GetActorLocation) (Variables|Controller|Bug|GetSpawnOffset)) (Transformation|GetActorRotation)))
  (bind _output_get (Variables|Private|SetPrimaryBug _spawnedbug))
  (EventDispatchers|AssignOnDeath (Class|FSDPawn|GetHealthComponent _output_get) (delegate Custom|PrimaryBugOnDeath))
  (Game|BindEventtoOnDestroyed (CallFunction|GetPrimaryBug) (delegate Custom|PrimaryBugDestroyed))
  (CallFunction|MULTIUpdateBugStats (CallFunction|GetPrimaryBug) (Variables|Controller|Bug|GetBugMoveSpeed) (Variables|Controller|Bug|GetBugTurnSpeed)))

(event Custom|SERVER_SummonSwarm
  (bind _swarmboundradius (Variables|Controller|Swarm|GetSwarmBoundRadius))
  (bind _root (Variables|Default|GetRoot))
  (bind _swarmboundradius_2 (Variables|Controller|Swarm|GetSwarmBoundRadius))
  (bind _returnvalue (Transformation|GetWorldLocation _root))
  (if (Variables|Controller|Swarm|GetCanSummonSwarm)
    (if (not (Variables|Private|GetIsDead))
      (Variables|Controller|Swarm|SetCanSummonSwarm false)
      (for _index (range 1 (Variables|Controller|Swarm|GetSwarmBugCount))
        (if (Variables|Controller|Swarm|GetIsSwarmFlying)
          (Variables|private|SetSwarmPos (CallFunction|RandomPointinSphere (Transformation|GetWorldLocation (Variables|Default|GetRoot)) _swarmboundradius_2 _swarmboundradius_2))
          (Variables|private|SetSpawnRot (Transformation|GetActorRotation (CallFunction|GetPrimaryBug)))
          (Variables|private|SetSwarmPos (+ (Variables|private|GetSwarmPos) (Variables|Controller|Swarm|GetSwarmSpawnOffset)) :!label _label)
          (bind _spawnedbug (CallFunction|SpawnSwarmBug (Variables|private|GetSwarmPos) (Variables|private|GetSpawnRot)))
          (Utilities|Map|Add (Variables|Private|GetBugFormationData) _spawnedbug (Utilities|Struct|MakeFBugFormationData (- (Variables|private|GetSwarmPos) _returnvalue)))
          (CallFunction|MULTIUpdateBugStats _spawnedbug (Variables|Controller|Bug|GetBugMoveSpeed) (Variables|Controller|Bug|GetBugTurnSpeed))
          (if (Variables|private|GetIsMoving)
            (Class|DeepPathfinderMovement|StartMoveto (Variables|/Script/FSD.DeepPathfinderCharacter|GetPathfinderMovement _spawnedbug) _returnvalue 25.0))
          (else
            (bind (_segmentstart _segmentend) (CallFunction|LineSegmentfromDirection (Math|Random|RandomPointinBoundingBox (+ (Transformation|GetWorldLocation (Variables|Default|GetRoot)) (* (Math|Vector|GetUpVector (Variables|Default|GetRoot)) 4e+02)) (Math|Vector|MakeVector _swarmboundradius _swarmboundradius 2e+02)) (* (Math|Vector|GetUpVector (Variables|Default|GetRoot)) -1.0) 1e+03))
            (bind (_outhit _returnvalue_2) (Collision|LineTraceByChannel _segmentstart _segmentend "TraceTypeQuery1" false (Utilities|Array|MakeArray self (Variables|Private|GetPrimaryBug)) "None"))
            (if _returnvalue_2
              (Variables|private|SetSwarmPos (.Location (Collision|BreakHitResult _outhit)))
              (Variables|private|SetSpawnRot (Math|Rotator|MakeRotfromZ (.Normal (Collision|BreakHitResult _outhit))))
              (goto _label)))))
      (Utilities|Time|SetTimerbyEvent (delegate Custom|SwarmCooldownEnd) (Variables|Controller|Swarm|GetSummonSwarmCooldown)))))

(event Custom|DestroyIfClientDenied
  (if (not (Variables|private|GetClientAccepted))
    (Actor|DestroyActor)))

(event Custom|EnableSecondaryAttack
  (Variables|Controller|BugAttacks|SetCanUseSecondaryAttack true))

(event Custom|EnableSwarmAttack
  (Variables|Controller|SwarmAttacks|SetCanUseSwarmAttack true))

(event Custom|EnablePrimaryAttack
  (Variables|Controller|BugAttacks|SetCanUsePrimaryAttack true))

(event Custom|SERVER_Suicide
  (for _array_element (CallFunction|GetAllBugs)
    (Utilities|IsValid _array_element
      (:Is%20Valid
        (if (not (Class|HealthComponentBase|IsDead (Class|FSDPawn|GetHealthComponent _array_element)))
          (Class|HealthComponentBase|Kill (Class|FSDPawn|GetHealthComponent _array_element) (CallFunction|GetPlayerPawn (Variables|Private|GetOwnerPlayer))))))))

(event Custom|SERVER_UpdateDestination
  (params (NewWorldDest :type Vector) (B :type Rotator))
  (Class|DeepPathfinderMovement|UpdateDestination (Variables|/Script/FSD.DeepPathfinderCharacter|GetPathfinderMovement (CallFunction|GetPrimaryBug)) NewWorldDest)
  (for _array_element (CallFunction|GetSwarmBugs)
    (Utilities|IsValid _array_element
      (:Is%20Valid
        (if (.ReturnValue (Utilities|Map|Find (Variables|Private|GetBugFormationData) _array_element))
          (Class|DeepPathfinderMovement|UpdateDestination (Variables|/Script/FSD.DeepPathfinderCharacter|GetPathfinderMovement _array_element) (select (Variables|Controller|Swarm|GetIsSwarmFlying) (+ NewWorldDest (Utilities|Struct|BreakFBugFormationData (.Value (Utilities|Map|Find (Variables|Private|GetBugFormationData) _array_element)))) (+ NewWorldDest (Math|Vector|MakeVector (.X (Math|Vector|BreakVector (Utilities|Struct|BreakFBugFormationData (.Value (Utilities|Map|Find (Variables|Private|GetBugFormationData) _array_element))))) (.Y (Math|Vector|BreakVector (Utilities|Struct|BreakFBugFormationData (.Value (Utilities|Map|Find (Variables|Private|GetBugFormationData) _array_element))))) 0.0)))))))))

(event Custom|PrimaryBugOnDeath
  (params (HealthComponent :type Health%20Component%20Base%20Object%20Reference))
  (CallFunction|BugDied))

(event Custom|SERVER_SwarmAttack
  (params (CameraTransform :type Transform))
  (if (Variables|Controller|SwarmAttacks|GetCanUseSwarmAttack)
    (for _array_element (CallFunction|GetSwarmBugs)
      (CallFunction|Attack _array_element (Variables|Controller|SwarmAttacks|GetSwarmAttackName) (Variables|Controller|SwarmAttacks|GetSwarmAttackRadius) (Variables|Controller|SwarmAttacks|GetSwarmAttackDistance) (Variables|Controller|SwarmAttacks|GetSwarmTargetingMethod) (Variables|Controller|SwarmAttacks|GetSwarmTargetingRule) CameraTransform))
    (Variables|Controller|SwarmAttacks|SetCanUseSwarmAttack false)
    (Utilities|Time|SetTimerbyEvent (delegate Custom|EnableSwarmAttack) (Variables|Controller|SwarmAttacks|GetSwarmAttackCooldown))))

(event Custom|SERVER_StartMove
  (params (Dest :type Vector%20%28by%20ref%29))
  (Class|DeepPathfinderMovement|StartMoveto (Variables|/Script/FSD.DeepPathfinderCharacter|GetPathfinderMovement (CallFunction|GetPrimaryBug)) Dest 25.0)
  (for _array_element (CallFunction|GetSwarmBugs)
    (Utilities|IsValid _array_element
      (:Is%20Valid
        (if (.ReturnValue (Utilities|Map|Find (Variables|Private|GetBugFormationData) _array_element))
          (Class|DeepPathfinderMovement|StartMoveto (Variables|/Script/FSD.DeepPathfinderCharacter|GetPathfinderMovement _array_element) (select (Variables|Controller|Swarm|GetIsSwarmFlying) (+ Dest (Utilities|Struct|BreakFBugFormationData (.Value (Utilities|Map|Find (Variables|Private|GetBugFormationData) _array_element)))) (+ Dest (Math|Vector|MakeVector (.X (Math|Vector|BreakVector (Utilities|Struct|BreakFBugFormationData (.Value (Utilities|Map|Find (Variables|Private|GetBugFormationData) _array_element))))) (.Y (Math|Vector|BreakVector (Utilities|Struct|BreakFBugFormationData (.Value (Utilities|Map|Find (Variables|Private|GetBugFormationData) _array_element))))) 0.0))) 5.0))))))

(event Custom|SERVER_SecondaryAttack
  (params (CameraTransform :type Transform))
  (if (Variables|Controller|BugAttacks|GetCanUseSecondaryAttack)
    (CallFunction|Attack (CallFunction|GetPrimaryBug) (Variables|Controller|BugAttacks|GetSecondaryAttackName) (Variables|Controller|BugAttacks|GetSecondaryAttackRadius) (Variables|Controller|BugAttacks|GetSecondaryAttackDistance) (Variables|Controller|BugAttacks|GetSecondaryTargetingMethod) (Variables|Controller|BugAttacks|GetSecondaryTargetingRule) CameraTransform)
    (Variables|Controller|BugAttacks|SetCanUseSecondaryAttack false)
    (Utilities|Time|SetTimerbyEvent (delegate Custom|EnableSecondaryAttack) (Variables|Controller|BugAttacks|GetSecondaryAttackCooldown))))

(event Custom|MULTI_UpdateBugStats
  (params (Bug :type Deep%20Pathfinder%20Character%20Object%20Reference) (Speed :type Float%20%28single-precision%29) (TurnSpeed :type Float%20%28single-precision%29))
  (bind _pathfindermovement (Variables|/Script/FSD.DeepPathfinderCharacter|GetPathfinderMovement Bug))
  (Class|DeepPathfinderMovement|SetMaxSpeed _pathfindermovement Speed)
  (Variables|/Script/FSD.DeepPathfinderMovement|SetAlignDirectionSpeed _pathfindermovement TurnSpeed))

(event Custom|SERVER_StopMove
  (Class|DeepPathfinderMovement|StopMove (Variables|/Script/FSD.DeepPathfinderCharacter|GetPathfinderMovement (CallFunction|GetPrimaryBug)))
  (if (Variables|Controller|Swarm|GetStopSwarmMovementInstantly)
    (for _array_element (CallFunction|GetSwarmBugs)
      (Class|DeepPathfinderMovement|StopMove (Variables|/Script/FSD.DeepPathfinderCharacter|GetPathfinderMovement _array_element))))
  (Variables|private|SetIsMoving false))

(event EventBeginPlay
  (bind _asplayer_controller (Utilities|Casting|CastToPlayerController (Components|GetOwner)))
  (Variables|Private|SetOwnerPlayer _asplayer_controller)
  (if (Networking|IsServer)
    (Utilities|Time|SetTimerbyEvent (delegate Custom|DestroyIfClientDenied) 5.0))
  (if (CallFunction|IsLocalBugController)
    (CallFunction|SERVERAcceptController)
    (bind _returnvalue (UserInterface|CreateWidget (Variables|Private|GetBugHudClass) (Variables|Private|GetOwnerPlayer) self))
    (bind _output_get (Variables|Private|SetBugHud _returnvalue))
    (UserInterface|Viewport|AddtoViewport _output_get 0)
    (CallFunction|SetViewTarget self)
    (CallFunction|SetPlayerInputEnabled false)
    (CallFunction|SetControllerInputEnabled true)
    (Actor|Tick|SetActorTickEnabled true)))

(event EventEndPlay
  (params (EndPlayReason :type EEndPlayReason%20Enum :default "Destroyed"))
  (if (Networking|IsServer)
    (if (Variables|private|GetClientAccepted)
      (CallFunction|SetPlayerGodMode false false false false)
      (CallFunction|SetPlayerLocation (Transformation|GetActorLocation (CallFunction|GetPrimaryBug)) true)
      (if (CallFunction|IsLocalBugController) :!label _label
        (Widget|RemovefromParent (Variables|Private|GetBugHud))
        (CallFunction|SetViewTarget (CallFunction|GetPlayerPawn (Variables|Private|GetOwnerPlayer)))
        (CallFunction|SetPlayerInputEnabled true)
        (CallFunction|SetControllerInputEnabled false)))
    (else
      (goto _label))))

(event EventTick
  (params (DeltaSeconds :type Float%20%28single-precision%29))
  (bind _rotationroot (Variables|Default|GetRotationRoot))
  (bind _relativerotation (Variables|/Script/Engine.SceneComponent|GetRelativeRotation _rotationroot))
  (Transformation|AddLocalRotation (Variables|Default|GetRotationRoot) (Math|Rotator|MakeRotator 0.0 (* (Class|Actor|GetInputAxisKeyValue) DeltaSeconds 175.0) (* (Class|Actor|GetInputAxisKeyValue) DeltaSeconds 8e+01)) false false)
  (Transformation|SetRelativeRotation (Variables|Default|GetRotationRoot) (Math|Rotator|MakeRotator 0.0 (Math|Float|Clamp(Float) (.pitch _relativerotation) -8e+01 8e+01) (.yaw _relativerotation)) false false)
  (if (Variables|private|GetLocalShouldMove)
    (CallFunction|SERVERUpdateDestination (Transformation|GetWorldLocation (Variables|Default|GetDest)) (Transformation|GetWorldRotation (Variables|Default|GetDest)))))

(event Input|KeyboardEvents|X
  (params (Key :type Key%20Structure :default "None"))
  (:Pressed
    (CallFunction|SERVERSuicide)))

(event Input|KeyboardEvents|W
  (params (Key :type Key%20Structure :default "None"))
  (:Pressed
    (Variables|private|SetLocalShouldMove true)
    (CallFunction|SERVERStartMove (Transformation|GetWorldLocation (Variables|Default|GetDest))))
  (:Released
    (Variables|private|SetLocalShouldMove false)
    (CallFunction|SERVERStopMove)))

(event Input|MouseEvents|LeftMouseButton
  (params (Key :type Key%20Structure :default "None"))
  (:Pressed
    (CallFunction|SERVERPrimaryAttack (Transformation|GetWorldTransform (Variables|Default|GetBugCamera)))))

(event Input|MouseEvents|RightMouseButton
  (params (Key :type Key%20Structure :default "None"))
  (:Pressed
    (CallFunction|SERVERSecondaryAttack (Transformation|GetWorldTransform (Variables|Default|GetBugCamera)))))

(event Input|KeyboardEvents|T
  (params (Key :type Key%20Structure :default "None"))
  (:Pressed
    (CallFunction|ToggleSpotlight)))

(event Input|KeyboardEvents|R
  (params (Key :type Key%20Structure :default "None"))
  (:Pressed
    (CallFunction|SERVERSummonSwarm)))

(event Input|MouseEvents|MiddleMouseButton
  (params (Key :type Key%20Structure :default "None"))
  (:Pressed
    (CallFunction|SERVERSwarmAttack (Transformation|GetWorldTransform (Variables|Default|GetBugCamera)))))

(fn ConstructionScript)

(fn IsLocalBugController
  (bind _returnvalue (CallFunction|GetLocalPlayer))
  (return (== _returnvalue (Variables|Private|GetOwnerPlayer))))

(fn GetPlayerPawn
  (params (Controller :type Controller%20Object%20Reference))
  (return (Pawn|GetControlledPawn Controller)))

(fn GetPrimaryBug
  (return (Variables|Private|GetPrimaryBug)))

(fn GetSwarmBugs
  (bind _keys (Utilities|Map|Keys (Variables|Private|GetBugFormationData)))
  (return _keys))

(fn GetAllBugs
  (Utilities|Array|Add (LocalVariables|GetBugsList) (CallFunction|GetPrimaryBug))
  (Utilities|Array|AppendArray (LocalVariables|GetBugsList) (CallFunction|GetSwarmBugs))
  (return (LocalVariables|GetBugsList)))

(fn GetAttackComponent
  (params (Bug :type Deep%20Pathfinder%20Character%20Object%20Reference) (ComponentName :type String))
  (for _array_element (Actor|GetComponentsByClass Bug "/Script/FSD.AttackBaseComponent")
    (if (Utilities|Enum|Equal(Enum) (Utilities|GetObjectName _array_element) ComponentName)
      (return _array_element))))

(fn SetPlayerGodMode
  (params (ReviveIfDown :type Boolean) (ResistsDamage :type Boolean) (HidePlayer :type Boolean) (IgnoreStatusEffects :type Boolean))
  (bind _ownerplayer (Variables|Private|GetOwnerPlayer))
  (bind _returnvalue (CallFunction|GetPlayerPawn _ownerplayer))
  (if ReviveIfDown
    (bind _asbp_player_character (Utilities|Casting|CastToBP_PlayerCharacter (CallFunction|GetPlayerPawn (Variables|Private|GetOwnerPlayer))))
    (Class|PlayerCharacter|ServerInstantRevive _asbp_player_character _asbp_player_character "Use"))
  (Class|HealthComponentBase|SetCanTakeDamage (Actor|GetComponentbyClass (CallFunction|GetPlayerPawn (Variables|Private|GetOwnerPlayer)) "/Script/FSD.PlayerHealthComponent") (not ResistsDamage))
  (Rendering|SetActorHiddenInGame _returnvalue HidePlayer)
  (Variables|/Script/FSD.StatusEffectsComponent|SetIgnoreAll (Actor|GetComponentbyClass _returnvalue "/Script/FSD.StatusEffectsComponent") IgnoreStatusEffects))

(fn SetPlayerLocation
  (params (NewLocation :type Vector) (PutOnGround :type Boolean))
  (bind _output_get (LocalVariables|SetDropLoc NewLocation))
  (if PutOnGround
    (bind (_segmentstart _segmentend) (CallFunction|LineSegmentfromDirection _output_get "0, 0,-1.000000" 5e+03))
    (bind (_outhit _returnvalue) (Collision|LineTraceByChannel _segmentstart _segmentend "TraceTypeQuery1" false (CallFunction|GetAllBugs) "None"))
    (if _returnvalue
      (LocalVariables|SetDropLoc (.Location (Collision|BreakHitResult _outhit)))))
  (Transformation|SetActorLocation (Pawn|GetControlledPawn (Variables|Private|GetOwnerPlayer)) (+ (LocalVariables|GetDropLoc) "0, 0,70.000000") false false))

(fn SetViewTarget
  (params (NewViewTarget :type Actor%20Object%20Reference))
  (Game|Player|SetViewTargetwithBlend (Variables|Private|GetOwnerPlayer) NewViewTarget 1.0 "VTBlend_Linear" 0.0 false))

(fn SetPlayerInputEnabled
  (params (NewEnabled :type Boolean))
  (bind _ownerplayer (Variables|Private|GetOwnerPlayer))
  (bind _ownerplayer_2 (Variables|Private|GetOwnerPlayer))
  (bind _returnvalue (CallFunction|GetPlayerPawn _ownerplayer_2))
  (if NewEnabled
    (Input|EnableInput _returnvalue _ownerplayer)
    (else
      (Input|DisableInput _returnvalue _ownerplayer))))

(fn SetControllerInputEnabled
  (params (NewEnabled :type Boolean))
  (bind _self self)
  (bind _ownerplayer (Variables|Private|GetOwnerPlayer))
  (if NewEnabled
    (Input|EnableInput _self _ownerplayer)
    (else
      (Input|DisableInput _self _ownerplayer))))

(fn SpawnBugAttached
  (params (WorldLocation :type Vector) (WorldRotation :type Rotator))
  (bind _returnvalue (Game|SpawnActorfromClass (Variables|Controller|Bug|GetBugClass) (Math|Transform|MakeTransform WorldLocation WorldRotation "1,1,1") "AlwaysSpawn" 0 0))
  (bind _asdeep_pathfinder_character (Utilities|Casting|CastToDeepPathfinderCharacter _returnvalue))
  (Pawn|UnPossess (Class|FSDPawn|GetFSDAIController _asdeep_pathfinder_character))
  (Transformation|AttachActorToActor self _asdeep_pathfinder_character "None" "SnapToTarget" "SnapToTarget" "KeepRelative" false)
  (return _asdeep_pathfinder_character))

(fn SpawnSwarmBug
  (params (WorldLocation :type Vector) (WorldRotation :type Rotator))
  (bind _returnvalue (Game|SpawnActorfromClass (Variables|Controller|Swarm|GetBugSwarmClass) (Math|Transform|MakeTransform WorldLocation WorldRotation "1,1,1") "AlwaysSpawn" 0 0))
  (bind _asdeep_pathfinder_character (Utilities|Casting|CastToDeepPathfinderCharacter _returnvalue))
  (Pawn|UnPossess (Class|FSDPawn|GetFSDAIController _asdeep_pathfinder_character))
  (return _asdeep_pathfinder_character))

(fn FindActorBestAngleOfAttack
  (params (MainActor :type Actor%20Object%20Reference) (Actors :type Array%20of%20Actor%20Object%20References))
  (for _array_element Actors
    (if (and (> (Class|Actor|GetDotProductto MainActor _array_element) (LocalVariables|GetBestAngle)) (> (Class|Actor|GetDotProductto MainActor _array_element) 0.0))
      (LocalVariables|SetBestAngle (Class|Actor|GetDotProductto MainActor _array_element))
      (LocalVariables|SetBestActor _array_element)))
  (return (LocalVariables|GetBestActor)))

(fn KillSwarm
  (for _array_element (CallFunction|GetSwarmBugs)
    (Utilities|IsValid _array_element
      (:Is%20Valid
        (if (not (Class|HealthComponentBase|IsDead (Class|FSDPawn|GetHealthComponent _array_element)))
          (Class|HealthComponentBase|Kill (Class|FSDPawn|GetHealthComponent _array_element) (CallFunction|GetPlayerPawn (Variables|Private|GetOwnerPlayer))))))))

(fn Attack
  (params (Bug :type Deep%20Pathfinder%20Character%20Object%20Reference) (AttackName :type String) (Radius :type Float%20%28single-precision%29) (Distance :type Float%20%28single-precision%29) (TargetingMethod :type EBugTargetingMethod%20Enum :default "NewEnumerator5") (TargetingRule :type EBugTargetingRule%20Enum :default "NewEnumerator0") (CameraTransform :type Transform))
  (Utilities|IsValid Bug
    (:Is%20Valid
      (bind _returnvalue (CallFunction|GetAttackComponent Bug AttackName))
      (LocalVariables|Setattackcomp _returnvalue)
      (bind _foundtargets (CallFunction|FindTargets Bug Radius Distance TargetingMethod TargetingRule CameraTransform))
      (if (> (Utilities|Array|Length _foundtargets) 0)
        (for _array_element _foundtargets
          (Class|AttackBaseComponent|AttackTarget (LocalVariables|Getattackcomp) _array_element))
        (else
          (Class|AttackBaseComponent|AttackTarget (LocalVariables|Getattackcomp)) ; This is a cosmetic attack when no bugs are around
        )))))

(fn ToggleSpotlight
  (Rendering|SetVisibility (Variables|Default|GetSpotLight) (not (Rendering|IsVisible (Variables|Default|GetSpotLight))) true))

(fn FindTargets
  (params (Bug :type Deep%20Pathfinder%20Character%20Object%20Reference) (Radius :type Float%20%28single-precision%29) (Distance :type Float%20%28single-precision%29) (TargetingMethod :type EBugTargetingMethod%20Enum :default "NewEnumerator5") (TargetingRule :type EBugTargetingRule%20Enum :default "NewEnumerator0") (CameraTransform :type Transform))
  (bind (_location _rotation) (Math|Transform|BreakTransform CameraTransform))
  (LocalVariables|SetCheckRadius Radius)
  (LocalVariables|SetTargetDistance Distance)
  (Utilities|IsValid Bug
    (:Is%20Valid
      (switch Utilities|FlowControl|Switch|SwitchonEBugTargetingMethod TargetingMethod
        (:NewEnumerator5
          (bind _segmentend (CallFunction|LineSegmentfromDirection (Transformation|GetActorLocation Bug) (Transformation|GetActorForwardVector Bug) (LocalVariables|GetTargetDistance)))
          (LocalVariables|SetTargetOrigin _segmentend)
          (bind (_outactors _returnvalue) (Collision|SphereOverlapActors (LocalVariables|GetTargetOrigin) (LocalVariables|GetCheckRadius) (LocalVariables|GetCheckTypes) "/Script/Engine.Pawn" (CallFunction|GetAllBugs) :!label _label))
          (LocalVariables|SetPotentialTargets _outactors)
          (if _returnvalue
            (switch Utilities|FlowControl|Switch|SwitchonEBugTargetingRule TargetingRule
              (:NewEnumerator0
                (Utilities|Array|AppendArray (LocalVariables|GetTargets) (LocalVariables|GetPotentialTargets)))
              (:NewEnumerator3
                (Utilities|Array|Add (LocalVariables|GetTargets) (.ReturnValue (Actor|FindNearestActor (Transformation|GetActorLocation Bug) (LocalVariables|GetPotentialTargets)))))
              (:NewEnumerator1
                (bind _returnvalue_2 (CallFunction|FindActorBestAngleOfAttack Bug (LocalVariables|GetPotentialTargets)))
                (Utilities|Array|Add (LocalVariables|GetTargets) _returnvalue_2)))
            (return (LocalVariables|GetTargets))))
        (:NewEnumerator0
          (bind (_segmentstart _segmentend_2) (CallFunction|LineSegmentfromDirection _location (Math|Vector|GetForwardVector _rotation) (LocalVariables|GetTargetDistance)))
          (bind (_outhit _returnvalue_3) (Collision|LineTraceByChannel _segmentstart _segmentend_2 "TraceTypeQuery1" false (CallFunction|GetAllBugs) "None"))
          (if _returnvalue_3
            (LocalVariables|SetTargetOrigin (.Location (Collision|BreakHitResult _outhit)))
            (goto _label)))))))