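; BP_GruntController is the Grunt-specific bug controller in the TwitchMod spawn module, adding server-side attacks on top of its parent's.
; Primary attack finds the best target within a radius of the direction arrow and passes it to the bug's attack component, falling back to the controller itself if none is found.
; Secondary attack casts the bug to the normal Spider Grunt and plays its alert scream.
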(event EventSERVERPrimaryAttack
  (bind _bugaspfc (Variables|Default|GetBugAsPFC))
  (bind _returnvalue (Actor|GetComponentbyClass _bugaspfc "/Script/FSD.AttackBaseComponent"))
  (|CallParentFunction)
  (bind _returnvalue_2 (CallFunction|FindBestTargetinRadius (Transformation|GetWorldLocation (Variables|Default|GetDirectionArrow)) 2e+02))
  (Utilities|IsValid _returnvalue_2
    (:Is%20Valid
      (Class|AttackBaseComponent|AttackTarget _returnvalue _returnvalue_2))
    (:Is%20Not%20Valid
      (Class|AttackBaseComponent|AttackTarget _returnvalue self))))

(event EventSERVERSecondaryAttack
  (|CallParentFunction)
  (bind _asene_spider_grunt_normal (Utilities|Casting|CastToENE_Spider_Grunt_Normal (Variables|Default|GetBugAsPFC)))
  (Default|AllPlayAlertScream _asene_spider_grunt_normal))

(fn ConstructionScript
  (|CallParentFunction))