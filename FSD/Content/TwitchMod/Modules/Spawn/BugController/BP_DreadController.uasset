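; Bug controller for the Dreadnought (spider tank boss) in the TwitchMod spawn module, mapping attack inputs to boss attacks.
; Primary and secondary server attack events run the parent logic, then find the best target in a radius around the Dest location.
; The controlled bug is cast to the spider tank boss, which fires its Fireball on primary and slam attack on secondary.
; A delayed slam-completion call is left unconnected.
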(event EventSERVERPrimaryAttack
  (|CallParentFunction)
  (bind _returnvalue (CallFunction|FindBestTargetinRadius (Transformation|GetWorldLocation (Variables|Default|GetDest)) 5e+02))
  (bind _asene_spider_tank_boss (Utilities|Casting|CastToENE_Spider_Tank_Boss (Variables|Default|GetBugAsPFC)))
  (Class|AttackBaseComponent|AttackTarget (Variables|/Game/Enemies/Spider/TankBoss/BossTank/ENE_Spider_Tank_Boss.ENE_Spider_Tank_Boss_C|Getfireball _asene_spider_tank_boss) _returnvalue))

(event EventSERVERSecondaryAttack
  (|CallParentFunction)
  (bind _returnvalue (CallFunction|FindBestTargetinRadius (Transformation|GetWorldLocation (Variables|Default|GetDest)) 4e+02))
  (bind _asene_spider_tank_boss (Utilities|Casting|CastToENE_Spider_Tank_Boss (Variables|Default|GetBugAsPFC)))
  (Class|AttackBaseComponent|AttackTarget (Variables|/Game/Enemies/Spider/TankBoss/BossTank/ENE_Spider_Tank_Boss.ENE_Spider_Tank_Boss_C|GetSlamAttackk _asene_spider_tank_boss) _returnvalue))

(fn ConstructionScript
  (|CallParentFunction))